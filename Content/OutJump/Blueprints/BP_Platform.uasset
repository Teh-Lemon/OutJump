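; BP_Platform is a scoring platform for OutJump that awards points the first time it is hit while active.
; The construction script randomly picks its type from a probability array, and SetPlatformType swaps the mesh material through a type-to-material map.
; A mesh hit calls Activate, which passes the type to the OutJumpGame game mode's AddScore, then switches the platform to the inactive type to prevent repeat scoring.
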(event `self.PlatformMesh.OnComponentHit`
  (params (HitComponent :type "PrimitiveComponent Object Reference") (OtherActor :type "Actor Object Reference") (OtherComp :type "PrimitiveComponent Object Reference") (NormalImpulse :type "Vector Structure") (Hit :type "HitResult Structure (by ref)"))
  (`self.Activate` self))

(fn `Activate`
  ;[1 1 1] Only if platform is active
  (if (`|EnumInequality` (`self.PlatformType`) "NewEnumerator2")
    ;[1 1 1] Add score to total
    (bind _asout_jump_game (cast `/Game/OutJump/Game/OutJumpGame` (`GameplayStatics.GetGameMode`))
      (:`then`
        (`/Game/OutJump/Game/OutJumpGame.AddScore` _asout_jump_game (`self.PlatformType`))
        ;[1 1 1] Deactivate platform
        (`self.SetPlatformType` self "NewEnumerator2"))
      (:`CastFailed`
        (`KismetSystemLibrary.PrintString` (`KismetStringLibrary.Concat_StrStr` "Cast to gamemode failed. Current mode: " (`KismetSystemLibrary.GetDisplayName` (`GameplayStatics.GetGameMode`))))))))

(fn `SetPlatformType`
  (params (NewType :type "/Game/OutJump/Game/EPlatformType Enum"))
  (bind _output_get (set `self.PlatformType` NewType))
  (`PrimitiveComponent.SetMaterial` (`self.PlatformMesh`) 0 (`BlueprintMapLibrary.Map_Find` (`self.MaterialTypes`) _output_get)))

(fn `UserConstructionScript`
  (bind _platformtypespawnprobabilities (`self.PlatformTypeSpawnProbabilities`))
  (`self.SetPlatformType` (`|GetArrayItem` _platformtypespawnprobabilities (`KismetMathLibrary.RandomIntegerInRange` 0 (`KismetArrayLibrary.Array_LastIndex` _platformtypespawnprobabilities)))))